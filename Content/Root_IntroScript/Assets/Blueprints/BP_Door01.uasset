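; BP_Door01 is a proximity door that slides open when the player character enters its collision volume and slides back when the player leaves.
; Overlap events check for Core_PlayerCharacter, set a PlayerInRange flag and play or reverse the TL_OpenDoor timeline.
; The timeline moves SMDoor in relative space by scaling EndPos and adding StartPos, so EndPos acts as an offset rather than a target position.
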(event OnComponentBeginOverlap(Collision)
  (params (OverlappedComponent :type Primitive%20Component%20Object%20Reference) (OtherActor :type Actor%20Object%20Reference) (OtherComp :type Primitive%20Component%20Object%20Reference) (OtherBodyIndex :type Integer) (bFromSweep :type Boolean) (SweepResult :type Hit%20Result%20Structure%20%28by%20ref%29))
  (Utilities|Casting|CastToCore_PlayerCharacter OtherActor)
  (Variables|Default|SetPlayerInRange true)
  (bind _newtrack_0 (Timeline|TL_OpenDoor Play)
    (:Update
      (Transformation|SetRelativeLocation (Variables|Default|GetSM_Door) (+ (* (Variables|Default|GetEndPos) _newtrack_0) (Variables|Default|GetStartPos)) false false))))

(event OnComponentEndOverlap(Collision)
  (params (OverlappedComponent :type Primitive%20Component%20Object%20Reference) (OtherActor :type Actor%20Object%20Reference) (OtherComp :type Primitive%20Component%20Object%20Reference) (OtherBodyIndex :type Integer))
  (Utilities|Casting|CastToCore_PlayerCharacter OtherActor)
  (Variables|Default|SetPlayerInRange false)
  (bind _newtrack_0 (Timeline|TL_OpenDoor Reverse)
    (:Update
      (Transformation|SetRelativeLocation (Variables|Default|GetSM_Door) (+ (* (Variables|Default|GetEndPos) _newtrack_0) (Variables|Default|GetStartPos)) false false))))

(fn ConstructionScript)