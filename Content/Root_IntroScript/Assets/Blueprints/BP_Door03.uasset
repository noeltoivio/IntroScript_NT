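; BP_Door03 is a door that slides toward an end position as soon as it starts ticking, with no trigger in its graph.
; On the first Tick, a DoOnce stores the Door component's relative location as the starting position.
; Every Tick then eases that position toward EndPos with VInterpTo and applies it to the Door without sweep, with no stop check.
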(event EventTick
  (params (DeltaSeconds :type Float%20%28single-precision%29))
  (Utilities|FlowControl|Sequence
    (:then_0
      (Utilities|FlowControl|DoOnce false
        (:Completed
          (Variables|Default|SetCurrentPos (Variables|/Script/Engine.SceneComponent|GetRelativeLocation (Variables|Default|GetDoor))))))
    (:then_1
      (bind _output_get (Variables|Default|SetCurrentPos (Math|Interpolation|VInterpTo (Variables|Default|GetCurrentPos) (Variables|Default|GetEndPos) (Utilities|Time|GetWorldDeltaSeconds) 2.0)))
      (Transformation|SetRelativeLocation (Variables|Default|GetDoor) _output_get false false))))

(fn ConstructionScript)